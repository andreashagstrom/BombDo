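; BombDo creature character that explodes with radial damage, fire particles and sound when it attacks, dies or runs out its lifetime.
; The server counts down TimesUp on Tick; expiry and the first attack type share an explosion path that also destroys the actor.
; On authority, a delayed BeginPlay reads game-mode INI options for population cap, timer, damage and metal-damaging type, destroying itself when the count exceeds the cap.
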(event Custom|Explosion
  (bind _returnvalue (Transformation|GetActorLocation))
  ;[1 1 1] Explosion event(used in BPDo Attack)
  (Utilities|FlowControl|Sequence
    (:then_0
      (Class|GameplayStatics|PlaySoundAttached "/Game/PrimalEarth/Sound/SFX/Dinos/Dragon/Dragon_FIre_Explosion_Cue.Dragon_Fire_Explosion_Cue" (Variables|Character|GetMesh))
      (bind _returnvalue_2 (Effects|SpawnEmitteratLocation "/Game/PrimalEarth/Effects/Particles/Fire/PS_C4AirExplosionFire_OLD.PS_C4AirExplosionFire_OLD" _returnvalue))
      (Transformation|SetRelativeScale3D _returnvalue_2 "15.000000,15.000000,15.000000")
      (Game|Damage|ApplyRadialDamage (Variables|Default|GetExplodeDamage) _returnvalue 1e+03 (Variables|Default|GetExplosionDamageType) 0 self 0 false "ECC_GameTraceChannel11" 0.0))
    (:then_1
      (Actor|DestroyActor))))

(event EventTick
  (params (DeltaSeconds :type Float%20%28single-precision%29))
  (bind _returnvalue (Transformation|GetActorLocation))
  ;[1 1 1] Tick logic for destroyed in time X
  (if (Networking|IsServer)
    (Variables|Default|SetTimesUp (- (Variables|Default|GetTimesUp) DeltaSeconds) false)
    (if (not (> (Variables|Default|GetTimesUp) 0.0))
      ;[1 1 1] Explosion event(used in BPDo Attack)
      (Utilities|FlowControl|Sequence
        (:then_0
          (Class|GameplayStatics|PlaySoundAttached "/Game/PrimalEarth/Sound/SFX/Dinos/Dragon/Dragon_FIre_Explosion_Cue.Dragon_Fire_Explosion_Cue" (Variables|Character|GetMesh))
          (bind _returnvalue_2 (Effects|SpawnEmitteratLocation "/Game/PrimalEarth/Effects/Particles/Fire/PS_C4AirExplosionFire_OLD.PS_C4AirExplosionFire_OLD" _returnvalue))
          (Transformation|SetRelativeScale3D _returnvalue_2 "15.000000,15.000000,15.000000")
          (Game|Damage|ApplyRadialDamage (Variables|Default|GetExplodeDamage) _returnvalue 1e+03 (Variables|Default|GetExplosionDamageType) 0 self 0 false "ECC_GameTraceChannel11" 0.0))
        (:then_1
          (Actor|DestroyActor))))))

(event EventBeginPlay
  ;[1 1 1] EBP Ini-options
  (|CallParentFunction)
  (Utilities|FlowControl|Delay 0.2)
  (Networking|SwitchHasAuthority
    (:Authority
      (bind _asshootergamemode (Utilities|Casting|CastToShooterGameMode (Game|GetGameMode)))
      (Utilities|FlowControl|Sequence
        (:then_0
          (bind _returnvalue (Class|ShooterGameMode|GetFloatOptionIni _asshootergamemode "BombDo" "MaxAllowed"))
          (if (<= (Math|Float|Floor _returnvalue) 0)
            (Variables|Default|SetMaxAllowed 150)
            (else
              (Variables|Default|SetMaxAllowed (Math|Float|Floor _returnvalue))))
          (bind _outactors (Actor|GetAllActorsOfClass "BombDo_Character_BP_C"))
          (for (_ _array_index) _outactors
            (if (not (< _array_index (Variables|Default|GetMaxAllowed)))
              (Actor|DestroyActor))))
        (:then_1
          (bind _returnvalue_2 (Class|ShooterGameMode|GetFloatOptionIni _asshootergamemode "BombDo" "PassiveExplodeTime"))
          (if (<= _returnvalue_2 0.0)
            (Variables|Default|SetTimesUp 1.8e+03 false)
            (else
              (Variables|Default|SetTimesUp _returnvalue_2 false))))
        (:then_2
          (bind _returnvalue_3 (Class|ShooterGameMode|GetFloatOptionIni _asshootergamemode "BombDo" "ExplodeDamage"))
          (if (<= _returnvalue_3 0.0)
            (Variables|Default|SetExplodeDamage 5e+01)
            (else
              (Variables|Default|SetExplodeDamage _returnvalue_3))))
        (:then_3
          (bind _returnvalue_4 (Class|ShooterGameMode|GetBoolOptionIni _asshootergamemode "BombDo" "ExplodeDamageMetal"))
          (if _returnvalue_4
            (Variables|Default|SetExplosionDamageType "/Game/PrimalEarth/CoreBlueprints/DamageTypes/DmgType_Explosion_Rocket.DmgType_Explosion_Rocket_C")
            (else
              (Variables|Default|SetExplosionDamageType (Variables|Default|GetExplosionDamageType)))))))))

(event EventOnSetDeath
  (bind _returnvalue (Transformation|GetActorLocation))
  ;[1 1 1] On death > Explosion
  (Class|GameplayStatics|PlaySoundAttached "/Game/PrimalEarth/Sound/SFX/Dinos/Dragon/Dragon_FIre_Explosion_Cue.Dragon_Fire_Explosion_Cue" (Variables|Character|GetMesh))
  (bind _returnvalue_2 (Effects|SpawnEmitteratLocation "/Game/PrimalEarth/Effects/Particles/Fire/PS_C4AirExplosionFire_OLD.PS_C4AirExplosionFire_OLD" _returnvalue))
  (Transformation|SetRelativeScale3D _returnvalue_2 "15.000000,15.000000,15.000000")
  (Game|Damage|ApplyRadialDamage (Variables|Default|GetExplodeDamage) _returnvalue 1e+03 (Variables|Default|GetExplosionDamageType) 0 self 0 false "ECC_GameTraceChannel11" 0.0))

(fn ConstructionScript
  (|CallParentFunction))

(fn BPDoAttack
  (params (AttackIndex :type Integer))
  (if (== AttackIndex 0)
    (if (Networking|IsServer)
      (CallFunction|Explosion))))