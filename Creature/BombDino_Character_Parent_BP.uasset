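; Parent creature Blueprint for BombDino characters that scales base stats from server ini multipliers.
; Shortly after BeginPlay, the authority reads each stat's multiplier from the "BombDo" section through ShooterGameMode, falling back to 1 when outside 1–1000.
; Each multiplier scales the matching maximum on the character status component; Health and Food also get their current values raised.
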(event EventBeginPlay
  ;[0.02994 0.635 0.0254] Stat modifier ini - https://blueprintue.com/blueprint/v7vz_m0j/
  (Utilities|FlowControl|Delay 0.2)
  (Networking|SwitchHasAuthority
    (:Authority
      (bind _asshootergamemode (Utilities|Casting|CastToShooterGameMode (Game|GetGameMode)))
      (bind _returnvalue (Class|ShooterGameMode|GetFloatOptionIni _asshootergamemode "BombDo" "HealthMultiplier"))
      (if (>= _returnvalue 1.0)
        (if (<= _returnvalue 1e+03)
          (Variables|Default|SetHealthMod _returnvalue)
          (else
            (Variables|Default|SetHealthMod 1.0 :!label _label)))
        (else
          (goto _label)))
      (bind _returnvalue_2 (Class|PrimalCharacter|GetCharacterStatusComponent))
      (Class|PrimalCharacterStatusComponent|SetMaxStatusValue _returnvalue_2 "Health" (* (Class|PrimalCharacterStatusComponent|BPGetMaxStatusValue _returnvalue_2 "Health") (Variables|Default|GetHealthMod)))
      (Class|PrimalCharacterStatusComponent|ModifyCurrentStatusValue _returnvalue_2 "Health" (* (Class|PrimalCharacterStatusComponent|BPGetMaxStatusValue _returnvalue_2 "Health") (Variables|Default|GetHealthMod)) false false false false 0 false false)
      (bind _returnvalue_3 (Class|ShooterGameMode|GetFloatOptionIni _asshootergamemode "BombDo" "StamMultiplier"))
      (if (>= _returnvalue_3 1.0)
        (if (<= _returnvalue_3 1e+03)
          (Variables|Default|SetStamMod _returnvalue_3)
          (else
            (Variables|Default|SetStamMod 1.0 :!label _label_2)))
        (else
          (goto _label_2)))
      (bind _returnvalue_4 (Class|PrimalCharacter|GetCharacterStatusComponent))
      (Class|PrimalCharacterStatusComponent|SetMaxStatusValue _returnvalue_4 "Stamina" (* (Class|PrimalCharacterStatusComponent|BPGetMaxStatusValue _returnvalue_4 "Stamina") (Variables|Default|GetStamMod)))
      (bind _returnvalue_5 (Class|ShooterGameMode|GetFloatOptionIni _asshootergamemode "BombDo" "WeightMultiplier"))
      (if (>= _returnvalue_5 1.0)
        (if (<= _returnvalue_5 1e+03)
          (Variables|Default|SetWeightMod _returnvalue_5)
          (else
            (Variables|Default|SetWeightMod 1.0 :!label _label_3)))
        (else
          (goto _label_3)))
      (bind _returnvalue_6 (Class|PrimalCharacter|GetCharacterStatusComponent))
      (Class|PrimalCharacterStatusComponent|SetMaxStatusValue _returnvalue_6 "Weight" (* (Class|PrimalCharacterStatusComponent|BPGetMaxStatusValue _returnvalue_6 "Weight") (Variables|Default|GetWeightMod)))
      (bind _returnvalue_7 (Class|ShooterGameMode|GetFloatOptionIni _asshootergamemode "BombDo" "DamageMultiplier"))
      (if (>= _returnvalue_7 1.0)
        (if (<= _returnvalue_7 1e+03)
          (Variables|Default|SetDamageMod _returnvalue_7)
          (else
            (Variables|Default|SetDamageMod 1.0 :!label _label_4)))
        (else
          (goto _label_4)))
      (bind _returnvalue_8 (Class|PrimalCharacter|GetCharacterStatusComponent))
      (Class|PrimalCharacterStatusComponent|SetMaxStatusValue _returnvalue_8 "MeleeDamageMultiplier" (* (Class|PrimalCharacterStatusComponent|BPGetMaxStatusValue _returnvalue_8 "MeleeDamageMultiplier") (Variables|Default|GetDamageMod)))
      (bind _returnvalue_9 (Class|ShooterGameMode|GetFloatOptionIni _asshootergamemode "BombDo" "SpeedMultiplier"))
      (if (>= _returnvalue_9 1.0)
        (if (<= _returnvalue_9 1e+03)
          (Variables|Default|SetSpeedMod _returnvalue_9)
          (else
            (Variables|Default|SetSpeedMod 1.0 :!label _label_5)))
        (else
          (goto _label_5)))
      (bind _returnvalue_10 (Class|PrimalCharacter|GetCharacterStatusComponent))
      (Class|PrimalCharacterStatusComponent|SetMaxStatusValue _returnvalue_10 "SpeedMultiplier" (* (Class|PrimalCharacterStatusComponent|BPGetMaxStatusValue _returnvalue_10 "SpeedMultiplier") (Variables|Default|GetSpeedMod)))
      (bind _returnvalue_11 (Class|ShooterGameMode|GetFloatOptionIni _asshootergamemode "BombDo" "CraftMultiplier"))
      (if (>= _returnvalue_11 1.0)
        (if (<= _returnvalue_11 1e+03)
          (Variables|Default|SetCraftMod _returnvalue_11)
          (else
            (Variables|Default|SetCraftMod 1.0 :!label _label_6)))
        (else
          (goto _label_6)))
      (bind _returnvalue_12 (Class|PrimalCharacter|GetCharacterStatusComponent))
      (Class|PrimalCharacterStatusComponent|SetMaxStatusValue _returnvalue_12 "CraftingSpeedMultiplier" (* (Class|PrimalCharacterStatusComponent|BPGetMaxStatusValue _returnvalue_12 "CraftingSpeedMultiplier") (Variables|Default|GetCraftMod)))
      (bind _returnvalue_13 (Class|ShooterGameMode|GetFloatOptionIni _asshootergamemode "BombDo" "FoodMultiplier"))
      (if (>= _returnvalue_13 1.0)
        (if (<= _returnvalue_13 1e+03)
          (Variables|Default|SetFoodMod _returnvalue_13)
          (else
            (Variables|Default|SetFoodMod 1.0 :!label _label_7)))
        (else
          (goto _label_7)))
      (bind _returnvalue_14 (Class|PrimalCharacter|GetCharacterStatusComponent))
      (Class|PrimalCharacterStatusComponent|SetMaxStatusValue _returnvalue_14 "Food" (* (Class|PrimalCharacterStatusComponent|BPGetMaxStatusValue _returnvalue_14 "Food") (Variables|Default|GetFoodMod)))
      (Class|PrimalCharacterStatusComponent|ModifyCurrentStatusValue _returnvalue_14 "Food" (* (Class|PrimalCharacterStatusComponent|BPGetMaxStatusValue _returnvalue_14 "Food") (Variables|Default|GetFoodMod)) false false false false 0 false false)
      (bind _returnvalue_15 (Class|ShooterGameMode|GetFloatOptionIni _asshootergamemode "BombDo" "TorpMultiplier"))
      (if (>= _returnvalue_15 1.0)
        (if (<= _returnvalue_15 1e+03)
          (Variables|Default|SetTorpMod _returnvalue_15)
          (else
            (Variables|Default|SetTorpMod 1.0 :!label _label_8)))
        (else
          (goto _label_8)))
      (bind _returnvalue_16 (Class|PrimalCharacter|GetCharacterStatusComponent))
      (Class|PrimalCharacterStatusComponent|SetMaxStatusValue _returnvalue_16 "Torpidity" (* (Class|PrimalCharacterStatusComponent|BPGetMaxStatusValue _returnvalue_16 "Torpidity") (Variables|Default|GetTorpMod))))))

(fn ConstructionScript
  (|CallParentFunction))